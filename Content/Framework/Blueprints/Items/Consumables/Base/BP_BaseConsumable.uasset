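; Base Blueprint for consumable items, extending a parent item class with the shared logic for using up an item.
; UseItem calls the parent, checks that the item data is usable and of the expected type, then runs ConsumeEffect on the character.
; If the effect succeeds, it removes one from the inventory and, on successful removal, destroys the actor and returns true.
; ConsumeEffect is a stub returning false, so nothing is consumed unless a child overrides it.
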(fn `ConsumeEffect`
  (params (ConsumingCharacter :type "/Game/Framework/Blueprints/Characters/BP_BaseCharacter Object Reference"))
  (returns (`Success?` :type Boolean))
  (return false))

(fn `UseItem`
  (params (UsingCharacter :type "/Game/Framework/Blueprints/Characters/BP_BaseCharacter Object Reference"))
  (returns (`bSuccess?` :type Boolean))
  (bind ((`CanBeUsed?_31_28DAB6A34750602FA5A79D94FEE3EE4B` _canbeused_) (`ItemType_23_DB94F1014FF175F447FC58A2F638E8AF` _itemtype)) (break `/Game/Framework/Blueprints/Data/Items/Struct_ItemData` (`self.ItemData`)))
  (`parent.UseItem` UsingCharacter)
  (if (and _canbeused_ (`|EnumEquality` _itemtype "NewEnumerator0"))
    (bind _success_ (`self.ConsumeEffect` (`self.Using Character`)))
    (if _success_
      (bind _success (`/Game/Framework/Blueprints/Components/BPC_Inventory.RemoveItemAtIndex` (`self.InventoryRef`) (`self.Index`) 1))
      (if _success
        (`self.K2_DestroyActor`)
        (return true)
        (else
          (return false)))
      (else
        _)))
  (return false))

(fn `UserConstructionScript`
  (`parent.UserConstructionScript`))